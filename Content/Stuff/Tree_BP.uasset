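; Tree actor that can be faded and made passable, using the "Opacity" material parameter on its static mesh.
; The Change event sets opacity, turning collision off and flagging the tree as faded unless the value is above its threshold.
; While faded, Tick overrides opacity by distance to the third-person player, more transparent when farther away, and prints the normalized distance for debugging.
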(event Custom|Change
  (params (NewParam :type Float%20%28double-precision%29))
  (bind _staticmesh (Variables|Default|GetStaticMesh))
  (Rendering|Material|SetScalarParameterValueonMaterials (Variables|Default|GetStaticMesh) "Opacity" NewParam)
  (if (> NewParam 0.7)
    (Collision|SetCollisionEnabled _staticmesh "QueryAndPhysics")
    (Variables|Default|SetFaded false)
    (else
      (Collision|SetCollisionEnabled _staticmesh "NoCollision")
      (Variables|Default|SetFaded true))))

(event EventBeginPlay)

(event Collision|EventActorBeginOverlap
  (params (OtherActor :type Actor%20Object%20Reference)))

(event EventTick
  (params (DeltaSeconds :type Float%20%28single-precision%29))
  (if (Variables|Default|GetFaded)
    (Rendering|Material|SetScalarParameterValueonMaterials (Variables|Default|GetStaticMesh) "Opacity" 0.0)
    (bind _asbp_third_person_character (Utilities|Casting|CastToBP_ThirdPersonCharacter (Game|GetPlayerCharacter 0)))
    (Rendering|Material|SetScalarParameterValueonMaterials (Variables|Default|GetStaticMesh) "Opacity" (Math|Float|Lerp 1.0 0.5 (Math|Float|NormalizetoRange (Math|Vector|VectorLength (- (Transformation|GetActorLocation) (Transformation|GetActorLocation _asbp_third_person_character))) 1e+02 2e+03)))
    (Development|PrintString (Utilities|String|ToString(Float) (Math|Float|NormalizetoRange (Math|Vector|VectorLength (- (Transformation|GetActorLocation) (Transformation|GetActorLocation _asbp_third_person_character))) 1e+02 2e+03)) true true "(R=0.000000,G=0.660000,B=1.000000,A=1.000000)" 0.0)))

(fn ConstructionScript)