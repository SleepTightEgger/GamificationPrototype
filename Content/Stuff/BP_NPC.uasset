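; BP_NPC is a talkable NPC that opens a dialogue screen for the player.
; Its sphere overlap registers it as the third-person character's NPC and shows a prompt widget; leaving clears the reference, though any actor's exit hides the widget.
; The Dialogue event disables player input, picks text from DialogueAsset using GS_Beneath's Generation and ForestRegion state, then shows WBP_Dialogue with cursor and UI-only input.
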(event OnComponentBeginOverlap(Sphere)
  (params (OverlappedComponent :type Primitive%20Component%20Object%20Reference) (OtherActor :type Actor%20Object%20Reference) (OtherComp :type Primitive%20Component%20Object%20Reference) (OtherBodyIndex :type Integer) (bFromSweep :type Boolean) (SweepResult :type Hit%20Result%20Structure%20%28by%20ref%29))
  (bind _returnvalue (Actor|GetActorOfClass "/Game/Stuff/BP_ThirdPersonCharacter.BP_ThirdPersonCharacter_C"))
  (if (== _returnvalue OtherActor)
    (Variables|/Game/Stuff/BP_ThirdPersonCharacter.BP_ThirdPersonCharacter_C|SetNPC _returnvalue self)
    (Rendering|SetVisibility (Variables|Default|GetWidget) true false)))

(event OnComponentEndOverlap(Sphere)
  (params (OverlappedComponent :type Primitive%20Component%20Object%20Reference) (OtherActor :type Actor%20Object%20Reference) (OtherComp :type Primitive%20Component%20Object%20Reference) (OtherBodyIndex :type Integer))
  (Rendering|SetVisibility (Variables|Default|GetWidget) false false)
  (bind _returnvalue (Actor|GetActorOfClass "/Game/Stuff/BP_ThirdPersonCharacter.BP_ThirdPersonCharacter_C"))
  (if (== _returnvalue OtherActor)
    (Variables|/Game/Stuff/BP_ThirdPersonCharacter.BP_ThirdPersonCharacter_C|SetNPC _returnvalue 0)))

(event Custom|Dialogue
  (params (Player :type BP%20Third%20Person%20Character%20Object%20Reference))
  (bind _returnvalue (Game|GetPlayerController 0))
  (bind _returnvalue_2 (Game|GetPlayerController 0))
  (Input|DisableInput (stale OnComponentBeginOverlap(Sphere) _returnvalue) _returnvalue)
  (bind _returnvalue_3 (UserInterface|CreateWidget "/Game/Stuff/Widgets/WBP_Dialogue.WBP_Dialogue_C" _returnvalue))
  (bind _asgs_beneath (Utilities|Casting|CastToGS_Beneath (Game|GetGameState)))
  (if (== (Variables|/Game/Stuff/Framework/GS_Beneath.GS_Beneath_C|GetGeneration _asgs_beneath) 2)
    (if (Variables|/Game/Stuff/Framework/GS_Beneath.GS_Beneath_C|GetForestRegion _asgs_beneath)
      (Variables|Default|SetDialogueIndex 2)
      (else
        (Variables|Default|SetDialogueIndex 1)))
    (else
      (Variables|Default|SetDialogueIndex 0)))
  (Default|SetText _returnvalue_3 (Variables|/Game/Stuff/Dialogue/DA_Dialogue.DA_Dialogue_C|GetDialogueText (Utilities|Array|Get(acopy) (Variables|Default|GetDialogueAsset) (Variables|Default|GetDialogueIndex))))
  (UserInterface|Viewport|AddtoViewport _returnvalue_3 0)
  (Variables|/Script/Engine.PlayerController|SetbShowMouseCursor _returnvalue_2 true)
  (Input|SetInputModeUIOnly _returnvalue_2 _returnvalue_3 "DoNotLock" false))

(event EventBeginPlay)

(event Collision|EventActorBeginOverlap
  (params (OtherActor :type Actor%20Object%20Reference)))

(event EventTick
  (params (DeltaSeconds :type Float%20%28single-precision%29)))

(fn ConstructionScript)